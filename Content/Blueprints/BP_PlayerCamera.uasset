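; Player camera that tracks the BP_DungeonRunner at fixed height and runs the card game used to affect dungeon traps.
; BeginPlay builds the draw pile and deals a hand of BP_Card actors laid out on HandAnchor.
; Selecting a card raises it and highlights valid floors; playing discards its data, with left-click here handling only Air placement.
; ClearBoard discards the hand, removes board cards and holograms, reactivates linked traps, frees floors and redeals.
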(event Custom|UpdateFloorHighlights
  (bind _outactors (Actor|GetAllActorsOfClass "/Game/Blueprints/Traps/BP_Floor.BP_Floor_C"))
  (for _array_element _outactors
    (bind _isvalid (Default|IsFloorValidforCard _array_element (Variables|/Game/Blueprints/Cards/BP_Card.BP_Card_C|GetCardData (Variables|Default|GetSelectedCard))))
    (if _isvalid
      (Default|ShowHighlight _array_element)
      (else
        (Default|HideHighlight _array_element)))))

(event Custom|ClearAllHighlights
  (bind _outactors (Actor|GetAllActorsOfClass "/Game/Blueprints/Traps/BP_Floor.BP_Floor_C"))
  (for _array_element _outactors
    (Default|HideHighlight _array_element)))

(event Custom|SelectCard
  (params (NewCard :type BP%20Card%20Object%20Reference))
  (Utilities|IsValid (Variables|Default|GetSelectedCard)
    (:Is%20Valid
      (Transformation|SetActorLocation (Variables|Default|GetSelectedCard) (Math|Vector|MakeVector (.x (Transformation|GetActorLocation (Variables|Default|GetSelectedCard))) (.y (Transformation|GetActorLocation (Variables|Default|GetSelectedCard))) (+ (.z (Transformation|GetActorLocation (Variables|Default|GetSelectedCard))) -3e+01)) false false))
    (:Is%20Not%20Valid
      _))
  (bind _output_get (Variables|Default|SetSelectedCard NewCard))
  (Transformation|SetActorLocation _output_get (Math|Vector|MakeVector (.x (Transformation|GetActorLocation _output_get)) (.y (Transformation|GetActorLocation _output_get)) (+ (.z (Transformation|GetActorLocation _output_get)) 3e+01)) false false)
  (CallFunction|UpdateFloorHighlights))

(event Custom|DeselectCard
  (Transformation|SetActorLocation (Variables|Default|GetSelectedCard) (Math|Vector|MakeVector (.x (Transformation|GetActorLocation (Variables|Default|GetSelectedCard))) (.y (Transformation|GetActorLocation (Variables|Default|GetSelectedCard))) (+ (.z (Transformation|GetActorLocation (Variables|Default|GetSelectedCard))) -3e+01)) false false)
  (Variables|Default|SetSelectedCard 0)
  (CallFunction|ClearAllHighlights))

(event Custom|PlaySelectedCard
  (params (TargetTransform :type Transform))
  (CallFunction|ClearAllHighlights)
  (Default|FlytoTarget (Variables|Default|GetSelectedCard) TargetTransform)
  (Utilities|Array|RemoveItem (Variables|Default|GetHand) (Variables|Default|GetSelectedCard))
  (Utilities|Array|Add (Variables|Default|GetDiscardPile) (Variables|/Game/Blueprints/Cards/BP_Card.BP_Card_C|GetCardData (Variables|Default|GetSelectedCard)))
  (Variables|Default|SetSelectedCard 0)
  (CallFunction|UpdateHandLayout))

(event Custom|ClearBoard
  (bind _activeboard (Variables|Default|GetActiveBoard))
  (CallFunction|DiscardHand)
  (for _array_element _activeboard
    (Utilities|IsValid _array_element
      (:Is%20Valid
        (Utilities|FlowControl|Sequence
          (:then_0
            (Utilities|IsValid (Variables|/Game/Blueprints/Cards/BP_Card.BP_Card_C|GetCardHologram _array_element)
              (:Is%20Valid
                (Actor|DestroyActor (Variables|/Game/Blueprints/Cards/BP_Card.BP_Card_C|GetCardHologram _array_element)))))
          (:then_1
            (Utilities|IsValid (Variables|/Game/Blueprints/Cards/BP_Card.BP_Card_C|GetLinkedTrap _array_element)
              (:Is%20Valid
                (Default|ActivateTrap (Variables|/Game/Blueprints/Cards/BP_Card.BP_Card_C|GetLinkedTrap _array_element)))))
          (:then_2
            (Actor|DestroyActor _array_element))))))
  (bind _outactors (Actor|GetAllActorsOfClass "/Game/Blueprints/Traps/BP_Floor.BP_Floor_C"))
  (for _array_element_2 _outactors
    (Variables|/Game/Blueprints/Traps/BP_Floor.BP_Floor_C|SetHasCard _array_element_2 false))
  (Utilities|Array|Clear _activeboard)
  (for _index (range 0 4)
    (CallFunction|DrawCard))
  (CallFunction|UpdateHandLayout))

(event Custom|ReshuffleDeck
  (bind _drawpile (Variables|Default|GetDrawPile))
  (bind _discardpile (Variables|Default|GetDiscardPile))
  (if (> (Utilities|Array|Length (Variables|Default|GetDiscardPile)) 0)
    (Utilities|Array|AppendArray _discardpile _drawpile)
    (Utilities|Array|Shuffle _drawpile)
    (Utilities|Array|Clear _discardpile)))

(event Custom|DrawCard
  (bind _drawpile (Variables|Default|GetDrawPile))
  (if (== (Utilities|Array|Length _drawpile) 0)
    (CallFunction|ReshuffleDeck)
    (else
      (Utilities|Array|RemoveIndex _drawpile)
      (bind _returnvalue (Game|SpawnActorfromClass "/Game/Blueprints/Cards/BP_Card.BP_Card_C" (Transformation|GetWorldTransform (Variables|Default|GetHandAnchor)) "Undefined" "MultiplyWithRoot" 0 (Utilities|Array|Get(acopy) _drawpile) 0))
      (Utilities|Array|Add (Variables|Default|GetHand) _returnvalue)
      (Transformation|AttachComponentToComponent _returnvalue (Variables|Default|GetHandAnchor) "None" "KeepWorld" "KeepWorld" "KeepWorld" true))))

(event Custom|UpdateHandLayout
  (bind _hand (Variables|Default|GetHand))
  (if (> (Utilities|Array|Length _hand) 0)
    (for (_array_element _array_index) _hand
      (Transformation|SetActorRelativeTransform _array_element (Math|Transform|MakeTransform (Math|Vector|MakeVector 0.0 (Math|Conversions|ToFloat(Integer) (* _array_index 60)) 0.0) "80.000000,0.000000,0.000000" "0.500000,0.500000,0.500000") false false)
      (Variables|/Game/Blueprints/Cards/BP_Card.BP_Card_C|SetHomeLocation _array_element (Transformation|GetActorLocation _array_element))
      (CallFunction|ClearAllHighlights))))

(event Custom|DiscardHand
  (bind _hand (Variables|Default|GetHand))
  (for _array_element _hand
    (Utilities|Array|Add (Variables|Default|GetDiscardPile) (Variables|/Game/Blueprints/Cards/BP_Card.BP_Card_C|GetCardData _array_element))
    (Actor|DestroyActor _array_element))
  (Utilities|Array|Clear _hand)
  (CallFunction|ReshuffleDeck))

(event EventBeginPlay
  (bind _returnvalue (Actor|GetActorOfClass "/Game/Blueprints/RunnerAI/BP_DungeonRunner.BP_DungeonRunner_C"))
  (Variables|Default|SetTargetAI _returnvalue)
  (for _index (range 0 5)
    (Utilities|Array|Add (Variables|Default|GetDrawPile) (Utilities|Struct|MakeF_CardData "Bridge" "/Game/Textures/Card6.Card6" "/Game/Blueprints/Holograms/BP_BridgeHologram.BP_BridgeHologram_C" "NewEnumerator1" "NewEnumerator2" "NewEnumerator1"))
    (Utilities|Array|Add (Variables|Default|GetDrawPile) (Utilities|Struct|MakeF_CardData "Block Flame" "/Game/Textures/Card5.Card5" "/Game/Blueprints/Holograms/BP_TrapBlockHologram.BP_TrapBlockHologram_C" "NewEnumerator1" "NewEnumerator2" "NewEnumerator4"))
    (Utilities|Array|Add (Variables|Default|GetDrawPile) (Utilities|Struct|MakeF_CardData "Block Spike" "/Game/Textures/Card3.Card3" "/Game/Blueprints/Holograms/BP_TrapBlockHologram.BP_TrapBlockHologram_C" "NewEnumerator1" "NewEnumerator2" "NewEnumerator2"))
    (Utilities|Array|Add (Variables|Default|GetDrawPile) (Utilities|Struct|MakeF_CardData "Stop Swing" "/Game/Textures/Card2.Card2" 0 "NewEnumerator1" "NewEnumerator2" "NewEnumerator6"))
    (Utilities|Array|Add (Variables|Default|GetDrawPile) (Utilities|Struct|MakeF_CardData "Empty" "/Engine/MobileResources/HUD/AnalogHat.AnalogHat" "/Game/Blueprints/Holograms/BP_TrapBlockHologram.BP_TrapBlockHologram_C" "NewEnumerator2" "NewEnumerator1"))
    (Utilities|Array|Add (Variables|Default|GetDrawPile) (Utilities|Struct|MakeF_CardData "Divine Shild" "/Game/Textures/Card1.Card1" "/Game/Blueprints/Holograms/BP_TrapBlockHologram.BP_TrapBlockHologram_C")))
  (for _index_2 (range 0 4)
    (CallFunction|DrawCard))
  (CallFunction|UpdateHandLayout))

(event EventTick
  (params (DeltaSeconds :type Float%20%28single-precision%29))
  (bind _targetai (Variables|Default|GetTargetAI))
  (bind _returnvalue (Transformation|GetActorLocation _targetai))
  (Utilities|IsValid (Variables|Default|GetTargetAI)
    (:Is%20Valid
      (Transformation|SetActorLocation (Math|Vector|MakeVector (.x _returnvalue) (.y _returnvalue) 2e+02) false false))))

(event Input|MouseEvents|LeftMouseButton
  (params (Key :type Key%20Structure :default "None"))
  (bind _returnvalue (Game|GetPlayerCameraManager 0))
  (bind _selectedcard (Variables|Default|GetSelectedCard))
  (:Pressed
    (Utilities|IsValid _selectedcard
      (:Is%20Valid
        (switch Utilities|FlowControl|Switch|SwitchonE_PlacementRule (.PlacementRule (Utilities|Struct|BreakF_CardData (Variables|/Game/Blueprints/Cards/BP_Card.BP_Card_C|GetCardData _selectedcard)))
          (:NewEnumerator0
            (bind _asbp_card (Utilities|Casting|CastToBP_Card (.HitActor (Collision|BreakHitResult (.HitResult (Game|Player|GetHitResultUnderCursorbyChannel (Game|GetPlayerController 0) "TraceTypeQuery1" true)))))
              (:CastFailed
                (CallFunction|PlaySelectedCard (Math|Transform|MakeTransform (+ (Camera|GetCameraLocation _returnvalue) (* (Math|Vector|GetForwardVector (Camera|GetCameraRotation _returnvalue)) 5e+02))))
                (Utilities|Array|AddUnique (Variables|Default|GetActiveBoard) _asbp_card)))))))))

(event Input|KeyboardEvents|1
  (params (Key :type Key%20Structure :default "None"))
  (:Pressed
    (CallFunction|DrawCard)
    (CallFunction|UpdateHandLayout)))

(fn ConstructionScript)