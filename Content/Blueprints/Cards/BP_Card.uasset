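; Playable card actor for a dungeon-runner game, with UI visuals from CardData, hover feedback and click selection through BP_PlayerCamera.
; CheckDropValidity traces under the cursor against the card's placement rule: air, empty ground or trap.
; FlyToTarget moves it by timeline lerp, then air cards apply shield or speed buffs to BP_DungeonRunner and vanish.
; Floor cards spawn an attached hologram, join the active board and deactivate any overlapped trap.
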(event OnClicked(StaticMesh)
  (params (TouchedComponent :type Primitive%20Component%20Object%20Reference) (ButtonPressed :type Key%20Structure :default "None"))
  (bind _self self)
  (bind _asbp_player_camera (Utilities|Casting|CastToBP_PlayerCamera (Game|Player|GetPlayerPawn 0)))
  (if (== (Variables|/Game/Blueprints/BP_PlayerCamera.BP_PlayerCamera_C|GetSelectedCard _asbp_player_camera) _self)
    (Default|DeselectCard _asbp_player_camera)
    (else
      (Default|SelectCard _asbp_player_camera _self)
      (Audio|PlaySoundatLocation "/Game/Sounds/CardSelect.CardSelect" (Transformation|GetActorLocation) "0, 0, 0" 1.0 1.0 0.0 0 0 0 0))))

(event OnBeginCursorOver(StaticMesh)
  (params (TouchedComponent :type Primitive%20Component%20Object%20Reference))
  (bind _asbp_player_camera (Utilities|Casting|CastToBP_PlayerCamera (Game|Player|GetPlayerPawn 0)))
  (if (not (== TouchedComponent (Variables|/Game/Blueprints/BP_PlayerCamera.BP_PlayerCamera_C|GetSelectedCard _asbp_player_camera)))
    (Rendering|Material|SetMaterial (Variables|Default|GetStaticMesh) 0 "/Game/Meshes/Card/MAT_SelectCard.MAT_SelectCard")
    (Audio|PlaySoundatLocation "/Game/Sounds/CardHover.CardHover" (Transformation|GetActorLocation) "0, 0, 0" 1.0 1.0 0.0 0 0 0 0)))

(event OnEndCursorOver(StaticMesh)
  (params (TouchedComponent :type Primitive%20Component%20Object%20Reference))
  (bind _asbp_player_camera (Utilities|Casting|CastToBP_PlayerCamera (Game|Player|GetPlayerPawn 0)))
  (if (not (== TouchedComponent (Variables|/Game/Blueprints/BP_PlayerCamera.BP_PlayerCamera_C|GetSelectedCard _asbp_player_camera)))
    (Rendering|Material|SetMaterial (Variables|Default|GetStaticMesh) 0 "/Game/Meshes/Card/MAT_Card.MAT_Card")))

(event Custom|FlyToTarget
  (params (TargetTransform :type Transform))
  (bind _returnvalue (Transformation|GetActorTransform))
  (bind _carddata (Variables|Default|GetCardData))
  (bind (_cardname _cardartwork _hologrambp _cardtype _placementrule _targettrap _bufftype _amount _buffvalue _duration) (Utilities|Struct|BreakF_CardData _carddata))
  (Transformation|DetachFromActor self "KeepWorld" "KeepWorld" "KeepWorld")
  (Collision|SetCollisionEnabled (Variables|Default|GetStaticMesh) "NoCollision")
  (bind _alpha (Timeline|Timeline Play)
    (:Update
      (Transformation|SetActorTransform (Math|Transform|MakeTransform (Math|Vector|MakeVector (.x (.location (Math|Transform|Lerp(Transform) (Transformation|GetActorTransform) TargetTransform _alpha))) (.y (.location (Math|Transform|Lerp(Transform) (Transformation|GetActorTransform) TargetTransform _alpha))) (- (.z (.location (Math|Transform|Lerp(Transform) (Transformation|GetActorTransform) TargetTransform _alpha))) 5.0)) (.rotation (Math|Transform|Lerp(Transform) (Transformation|GetActorTransform) TargetTransform _alpha)) (.scale (Math|Transform|Lerp(Transform) (Transformation|GetActorTransform) TargetTransform _alpha)))))
    (:Finished
      (switch Utilities|FlowControl|Switch|SwitchonE_PlacementRule _placementrule
        (:NewEnumerator0
          (switch Utilities|FlowControl|Switch|SwitchonE_BuffType _bufftype
            (:NewEnumerator1
              (Actor|DestroyActor))
            (:NewEnumerator0
              (bind _returnvalue_2 (Actor|GetActorOfClass "/Game/Blueprints/RunnerAI/BP_DungeonRunner.BP_DungeonRunner_C"))
              (Default|ApplyShieldBuff _returnvalue_2)
              (Actor|DestroyActor))
            (:NewEnumerator2
              (bind _returnvalue_3 (Actor|GetActorOfClass "/Game/Blueprints/RunnerAI/BP_DungeonRunner.BP_DungeonRunner_C"))
              (Default|ApplySpeedEffect _returnvalue_3 _buffvalue _duration)
              (Actor|DestroyActor))))
        (:NewEnumerator1
          (if (Utilities|IsValidClass _hologrambp) :!label _label
            (bind _returnvalue_4 (Game|SpawnActorfromClass _hologrambp (Math|Transform|MakeTransform (Math|Vector|MakeVector (.x (.location _returnvalue)) (.y (.location _returnvalue)) (- (.z (.location _returnvalue)) 5.0)) (.rotation _returnvalue) "1.000000,1.000000,1.000000") "Undefined" "MultiplyWithRoot" 0 0))
            (bind _output_get (Variables|Default|SetCardHologram _returnvalue_4))
            (Transformation|AttachActorToActor _output_get self "None" "KeepWorld" "KeepWorld" "KeepWorld" true))
          (bind _asbp_player_camera (Utilities|Casting|CastToBP_PlayerCamera (Game|Player|GetPlayerPawn 0)))
          (Utilities|Array|AddUnique (Variables|/Game/Blueprints/BP_PlayerCamera.BP_PlayerCamera_C|GetActiveBoard _asbp_player_camera) self)
          (bind _outactors (Collision|SphereOverlapActors (Transformation|GetActorLocation) 1e+01 (Utilities|Array|MakeArray "ObjectTypeQuery2") "/Game/Blueprints/Traps/BP_BaseTrap.BP_BaseTrap_C"))
          (bind _asbp_base_trap (Utilities|Casting|CastToBP_BaseTrap (Utilities|Array|Get(acopy) _outactors)))
          (bind _output_get_2 (Variables|Default|SetLinkedTrap _asbp_base_trap))
          (Default|DeactivateTrap _output_get_2))
        (:NewEnumerator2
          (goto _label))))))

(event EventBeginPlay
  (bind _aswbp_card_ui (Utilities|Casting|CastToWBP_CardUI (UserInterface|GetUserWidgetObject (Variables|Default|GetWidget))))
  (Default|UpdateCardVisuals _aswbp_card_ui (Variables|Default|GetCardData)))

(fn ConstructionScript)

(fn SetTargetLocation
  (switch Utilities|FlowControl|Switch|SwitchonE_PlacementRule (.PlacementRule (Utilities|Struct|BreakF_CardData (Variables|Default|GetCardData)))))

(fn CheckDropValidity
  (bind _returnvalue (Game|GetPlayerController 0))
  (bind _hitresult (Game|Player|GetHitResultUnderCursorbyChannel _returnvalue "TraceTypeQuery1" true))
  (bind _hitactor (Collision|BreakHitResult _hitresult))
  (switch Utilities|FlowControl|Switch|SwitchonE_PlacementRule (.PlacementRule (Utilities|Struct|BreakF_CardData (Variables|Default|GetCardData)))
    (:NewEnumerator0
      (return true))
    (:NewEnumerator1
      (Utilities|Casting|CastToBP_BaseTrap _hitactor
        (:CastFailed
          (if (Actor|ActorHasTag _hitactor "Ground")
            (return true)))))
    (:NewEnumerator2
      (Utilities|Casting|CastToBP_BaseTrap _hitactor)
      (return true))))