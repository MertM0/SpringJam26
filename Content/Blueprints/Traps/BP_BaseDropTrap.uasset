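; Base drop trap that fires when a BP_DungeonRunner enters its trigger zone, unless deactivated.
; A timeline slides DamageZone along local Z with a cage sound, and a second timeline reverses it after a delay.
; A shielded runner also switches off FallingObject collision, restored when the reverse finishes.
; DamageZone overlap deals TrapDamage and disables the runner's spring arm collision test.
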(event OnComponentBeginOverlap(TriggerZone)
  (params (OverlappedComponent :type Primitive%20Component%20Object%20Reference) (OtherActor :type Actor%20Object%20Reference) (OtherComp :type Primitive%20Component%20Object%20Reference) (OtherBodyIndex :type Integer) (bFromSweep :type Boolean) (SweepResult :type Hit%20Result%20Structure%20%28by%20ref%29))
  (bind _asbp_dungeon_runner (Utilities|Casting|CastToBP_DungeonRunner OtherActor))
  (if (not (Variables|Default|GetIsDeactivated))
    (if (Variables|/Game/Blueprints/RunnerAI/BP_DungeonRunner.BP_DungeonRunner_C|GetHasShield _asbp_dungeon_runner)
      (Collision|SetCollisionEnabled (Variables|Default|GetFallingObject) "NoCollision")
      (bind _spikemove (Timeline|Timeline PlayFromStart)
        (:Update
          (Transformation|SetRelativeLocation (Variables|Default|GetDamageZone) (Math|Vector|Lerp(Vector) "0.000000,0.000000,10.000000" "0.000000,0.000000,250.000000" _spikemove) false false)
          (Utilities|FlowControl|Delay 1.0)
          (bind _spikemove_2 (Timeline|Timeline_0 ReverseFromEnd)
            (:Update
              (Transformation|SetRelativeLocation (Variables|Default|GetDamageZone) (Math|Vector|Lerp(Vector) "0.000000,0.000000,10.000000" "0.000000,0.000000,250.000000" _spikemove_2) false false))
            (:Finished
              (Collision|SetCollisionEnabled (Variables|Default|GetFallingObject) "QueryAndPhysics"))))
        (:Event
          (Audio|PlaySoundatLocation "/Game/Sounds/Cage.Cage" (Transformation|GetActorLocation) "0, 0, 0" 1.0 1.0 0.0 "/Game/Sounds/SA_TrapSounds.SA_TrapSounds" 0 0 0)))
      (else
        (Timeline|Timeline PlayFromStart)))))

(event OnComponentBeginOverlap(DamageZone)
  (params (OverlappedComponent :type Primitive%20Component%20Object%20Reference) (OtherActor :type Actor%20Object%20Reference) (OtherComp :type Primitive%20Component%20Object%20Reference) (OtherBodyIndex :type Integer) (bFromSweep :type Boolean) (SweepResult :type Hit%20Result%20Structure%20%28by%20ref%29))
  (bind _asbp_dungeon_runner (Utilities|Casting|CastToBP_DungeonRunner OtherActor))
  (Default|TakeDamage _asbp_dungeon_runner (Variables|Default|GetTrapDamage))
  (Variables|/Script/Engine.SpringArmComponent|SetbDoCollisionTest (Variables|/Game/Blueprints/RunnerAI/BP_DungeonRunner.BP_DungeonRunner_C|GetSpringArm _asbp_dungeon_runner) false))

(fn ConstructionScript
  (|CallParentFunction))