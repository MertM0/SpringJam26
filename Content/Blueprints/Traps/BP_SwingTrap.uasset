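; Swinging blade trap, a child of a parent trap class, that damages the dungeon runner on contact.
; The T_Swing timeline starts on BeginPlay or activation, sweeps blade pitch back and forth with swing sounds, and parks it to one side when deactivated.
; BladeDamage overlap applies TrapDamage, plays a hit sound, clears CanDamage and disables DamageZone collision.
; The logic restoring BladeDamage collision and CanDamage is unwired.
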(event OnComponentBeginOverlap(BladeDamage)
  (params (OverlappedComponent :type Primitive%20Component%20Object%20Reference) (OtherActor :type Actor%20Object%20Reference) (OtherComp :type Primitive%20Component%20Object%20Reference) (OtherBodyIndex :type Integer) (bFromSweep :type Boolean) (SweepResult :type Hit%20Result%20Structure%20%28by%20ref%29))
  (bind _asbp_dungeon_runner (Utilities|Casting|CastToBP_DungeonRunner OtherActor))
  (Default|TakeDamage _asbp_dungeon_runner (Variables|Default|GetTrapDamage))
  (Audio|PlaySoundatLocation "/Game/Sounds/AxeHit.AxeHit" (Transformation|GetActorLocation) "0, 0, 0" 1.0 1.0 0.0 "/Game/Sounds/SA_TrapSounds.SA_TrapSounds" 0 0 0)
  (Variables|Default|SetCanDamage false)
  (Collision|SetCollisionEnabled (Variables|Default|GetDamageZone) "NoCollision"))

(event EventActivateTrap
  (|CallParentFunction)
  (bind _alpha (Timeline|T_Swing Play)
    (:Update
      (if (Variables|Default|GetIsDeactivated)
        (Transformation|SetRelativeRotation (Variables|Default|GetSM_PROP_trap_blade_dungeon_02) (Math|Rotator|MakeRotator 0.0 6e+01 0.0) false false)
        (Timeline|T_Swing Stop)
        (else
          (Transformation|SetRelativeRotation (Variables|Default|GetSM_PROP_trap_blade_dungeon_02) (Math|Rotator|MakeRotator 0.0 (Math|Float|Lerp -6e+01 6e+01 _alpha) 0.0) false false))))
    (:PlaySound
      (Audio|PlaySoundatLocation "/Game/Sounds/AxeSwing.AxeSwing" (Transformation|GetActorLocation) "0, 0, 0" 1.0 1.0 0.0 "/Game/Sounds/SA_TrapSounds.SA_TrapSounds" 0 0 0))))

(event EventBeginPlay
  (bind _alpha (Timeline|T_Swing Play)
    (:Update
      (if (Variables|Default|GetIsDeactivated)
        (Transformation|SetRelativeRotation (Variables|Default|GetSM_PROP_trap_blade_dungeon_02) (Math|Rotator|MakeRotator 0.0 6e+01 0.0) false false)
        (Timeline|T_Swing Stop)
        (else
          (Transformation|SetRelativeRotation (Variables|Default|GetSM_PROP_trap_blade_dungeon_02) (Math|Rotator|MakeRotator 0.0 (Math|Float|Lerp -6e+01 6e+01 _alpha) 0.0) false false))))
    (:PlaySound
      (Audio|PlaySoundatLocation "/Game/Sounds/AxeSwing.AxeSwing" (Transformation|GetActorLocation) "0, 0, 0" 1.0 1.0 0.0 "/Game/Sounds/SA_TrapSounds.SA_TrapSounds" 0 0 0))))

(fn ConstructionScript
  (|CallParentFunction))