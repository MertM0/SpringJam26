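; BP_BaseTrap is a base trap Blueprint with a DamageZone and an on/off state.
; DeactivateTrap sets the IsDeactivated flag, disables the zone's collision and plays a deactivation sound at the trap's location.
; ActivateTrap clears the flag, restores query-only collision and sets HasCard to false on its Floor reference.
; The DamageZone overlap event is empty, so this Blueprint applies no damage itself.
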(event OnComponentBeginOverlap(DamageZone)
  (params (OverlappedComponent :type Primitive%20Component%20Object%20Reference) (OtherActor :type Actor%20Object%20Reference) (OtherComp :type Primitive%20Component%20Object%20Reference) (OtherBodyIndex :type Integer) (bFromSweep :type Boolean) (SweepResult :type Hit%20Result%20Structure%20%28by%20ref%29)))

(event Custom|ActivateTrap
  (Variables|Default|SetIsDeactivated false)
  (Collision|SetCollisionEnabled (Variables|Default|GetDamageZone) "QueryOnly")
  (Variables|/Game/Blueprints/Traps/BP_Floor.BP_Floor_C|SetHasCard (Variables|Default|GetFloor) false))

(event Custom|DeactivateTrap
  (Variables|Default|SetIsDeactivated true)
  (Collision|SetCollisionEnabled (Variables|Default|GetDamageZone) "NoCollision")
  (Audio|PlaySoundatLocation "/Game/Sounds/TrapDeactivite.TrapDeactivite" (Transformation|GetActorLocation) "0, 0, 0" 1.0 1.0 0.0 0 0 0 0))

(fn ConstructionScript)