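; BP_Floor is a floor tile that hosts an optional trap and serves as a placement target for cards.
; On BeginPlay it spawns the pit, spear, flame, cage drop or swing trap matching CurrentTrapType, attaches it to TrapPoint and passes itself as Floor.
; Clicking its toggleable Highlight plays BP_PlayerCamera's selected card slightly above the tile if IsFloorValidForCard accepts its placement rule, then marks the tile occupied.
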(event OnClicked(Highlight)
  (params (TouchedComponent :type Primitive%20Component%20Object%20Reference) (ButtonPressed :type Key%20Structure :default "None"))
  (bind _returnvalue (Transformation|GetActorTransform))
  (bind _asbp_player_camera (Utilities|Casting|CastToBP_PlayerCamera (Game|Player|GetPlayerPawn 0)))
  (Utilities|IsValid (Variables|/Game/Blueprints/BP_PlayerCamera.BP_PlayerCamera_C|GetSelectedCard _asbp_player_camera)
    (:Is%20Valid
      (bind _isvalid (CallFunction|IsFloorValidforCard (Variables|/Game/Blueprints/Cards/BP_Card.BP_Card_C|GetCardData (Variables|/Game/Blueprints/BP_PlayerCamera.BP_PlayerCamera_C|GetSelectedCard _asbp_player_camera))))
      (if _isvalid
        (Default|PlaySelectedCard _asbp_player_camera (Math|Transform|MakeTransform (Math|Vector|MakeVector (.x (.location _returnvalue)) (.y (.location _returnvalue)) (+ (.z (.location _returnvalue)) 7.0)) (.rotation _returnvalue) (.scale _returnvalue)))
        (Variables|Default|SetHasCard true)))))

(event Custom|HideHighlight
  (Rendering|SetVisibility (Variables|Default|GetHighlight) false false))

(event Custom|ShowHighlight
  (Rendering|SetVisibility (Variables|Default|GetHighlight) true false))

(event EventBeginPlay
  (bind _trappoint (Variables|Default|GetTrapPoint))
  (bind _returnvalue (Transformation|GetRelativeTransform _trappoint))
  (switch Utilities|FlowControl|Switch|SwitchonE_TrapType (Variables|Default|GetCurrentTrapType)
    (:NewEnumerator1
      (bind _returnvalue_2 (Game|SpawnActorfromClass "/Game/Blueprints/Traps/BP_PitTrap.BP_PitTrap_C" (Math|Transform|MakeTransform (.location _returnvalue) (.rotation _returnvalue) "1.000000,1.000000,1.000000") "Undefined" "MultiplyWithRoot" 0 0))
      (Transformation|AttachComponentToComponent _returnvalue_2 (Variables|Default|GetTrapPoint) "None" "KeepRelative" "KeepRelative" "KeepRelative" true)
      (Variables|/Game/Blueprints/Traps/BP_BaseTrap.BP_BaseTrap_C|SetFloor _returnvalue_2 self))
    (:NewEnumerator2
      (bind _returnvalue_3 (Game|SpawnActorfromClass "/Game/Blueprints/Traps/BP_SpearTrap.BP_SpearTrap_C" (Math|Transform|MakeTransform (.location _returnvalue) (.rotation _returnvalue) "1.000000,1.000000,1.000000") "Undefined" "MultiplyWithRoot" 0 0))
      (Transformation|AttachComponentToComponent _returnvalue_3 (Variables|Default|GetTrapPoint) "None" "KeepRelative" "KeepRelative" "KeepRelative" true)
      (Variables|/Game/Blueprints/Traps/BP_BaseTrap.BP_BaseTrap_C|SetFloor _returnvalue_3 self))
    (:NewEnumerator4
      (bind _returnvalue_4 (Game|SpawnActorfromClass "/Game/Blueprints/Traps/BP_FlameTrap.BP_FlameTrap_C" (Math|Transform|MakeTransform (.location _returnvalue) (.rotation _returnvalue) "1.000000,1.000000,1.000000") "Undefined" "MultiplyWithRoot" 0 0))
      (Transformation|AttachComponentToComponent _returnvalue_4 (Variables|Default|GetTrapPoint) "None" "KeepRelative" "KeepRelative" "KeepRelative" true)
      (Variables|/Game/Blueprints/Traps/BP_BaseTrap.BP_BaseTrap_C|SetFloor _returnvalue_4 self))
    (:NewEnumerator5
      (bind _returnvalue_5 (Game|SpawnActorfromClass "/Game/Blueprints/Traps/BP_CageDropTrap.BP_CageDropTrap_C" (Math|Transform|MakeTransform (.location _returnvalue) (.rotation _returnvalue) "1.000000,1.000000,1.000000") "Undefined" "MultiplyWithRoot" 0 0))
      (Transformation|AttachComponentToComponent _returnvalue_5 (Variables|Default|GetTrapPoint) "None" "KeepRelative" "KeepRelative" "KeepRelative" true)
      (Variables|/Game/Blueprints/Traps/BP_BaseTrap.BP_BaseTrap_C|SetFloor _returnvalue_5 self))
    (:NewEnumerator6
      (bind _returnvalue_6 (Game|SpawnActorfromClass "/Game/Blueprints/Traps/BP_SwingTrap.BP_SwingTrap_C" (Math|Transform|MakeTransform (.location _returnvalue) (.rotation _returnvalue) "1.000000,1.000000,1.000000") "Undefined" "MultiplyWithRoot" 0 0))
      (Transformation|AttachComponentToComponent _returnvalue_6 (Variables|Default|GetTrapPoint) "None" "KeepRelative" "KeepRelative" "KeepRelative" true)
      (Variables|/Game/Blueprints/Traps/BP_BaseTrap.BP_BaseTrap_C|SetFloor _returnvalue_6 self))))

(fn ConstructionScript)

(fn IsFloorValidforCard
  (params (CardData :type F%20Card%20Data%20Structure))
  (bind (_cardname _cardartwork _hologrambp _cardtype _placementrule _targettrap) (Utilities|Struct|BreakF_CardData CardData))
  (if (Variables|Default|GetHasCard)
    (return false)
    (else
      (switch Utilities|FlowControl|Switch|SwitchonE_PlacementRule _placementrule
        (:NewEnumerator0
          (return false))
        (:NewEnumerator1
          (return (Utilities|Enum|Equal(Enum) (Variables|Default|GetCurrentTrapType) "NewEnumerator0")))
        (:NewEnumerator2
          (return (Utilities|Enum|Equal(Enum) _targettrap (Variables|Default|GetCurrentTrapType))))))))