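; Dungeon flame trap that erupts on a looping timer and damages BP_DungeonRunner actors entering its damage zone.
; Each eruption activates five Niagara fire effects, enables query collision after a short delay, then shuts both off.
; When IsDeactivated is set, timer ticks only switch off fire and collision.
; Damage comes solely from begin-overlap events; the loop over already overlapping actors has an empty body.
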(event OnComponentBeginOverlap(DamageZone)
  (params (OverlappedComponent :type Primitive%20Component%20Object%20Reference) (OtherActor :type Actor%20Object%20Reference) (OtherComp :type Primitive%20Component%20Object%20Reference) (OtherBodyIndex :type Integer) (bFromSweep :type Boolean) (SweepResult :type Hit%20Result%20Structure%20%28by%20ref%29))
  (bind _asbp_dungeon_runner (Utilities|Casting|CastToBP_DungeonRunner OtherActor))
  (Default|TakeDamage _asbp_dungeon_runner (Variables|Default|GetTrapDamage)))

(event Custom|EruptFlames
  (if (Variables|Default|GetIsDeactivated)
    (Components|Activation|Deactivate (Variables|Default|GetPS_FX_fire_dungeon_02_Niagara))
    (Collision|SetCollisionEnabled (Variables|Default|GetDamageZone) "NoCollision")
    (else
      (Components|Activation|SetActive (Variables|Default|GetPS_FX_fire_dungeon_02_Niagara4) true true)
      (Utilities|FlowControl|Delay 0.5)
      (Collision|SetCollisionEnabled (Variables|Default|GetDamageZone) "QueryOnly")
      (for _array_element (Collision|GetOverlappingActors (Variables|Default|GetDamageZone) 0 :!class /Script/Engine.PrimitiveComponent)
        _)
      (Utilities|FlowControl|Delay 2.0)
      (Components|Activation|Deactivate (Variables|Default|GetPS_FX_fire_dungeon_02_Niagara))
      (Collision|SetCollisionEnabled (Variables|Default|GetDamageZone) "NoCollision"))))

(event EventBeginPlay
  (Utilities|Time|SetTimerbyEvent (delegate Custom|EruptFlames) 4.0 true)
  (Collision|SetCollisionEnabled (Variables|Default|GetDamageZone) "NoCollision"))

(fn ConstructionScript
  (|CallParentFunction))