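; Spear trap that hurts the dungeon runner when triggered.
; A runner entering TriggerZone plays a timeline that moves DamageZone vertically, unless the trap is deactivated.
; DamageZone overlap applies TrapDamage to the runner through a DoOnce that resets after a short delay, limiting repeated hits.
; The deactivation flag gates only the movement, as the damage overlap does not check it.
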(event OnComponentBeginOverlap(TriggerZone)
  (params (OverlappedComponent :type Primitive%20Component%20Object%20Reference) (OtherActor :type Actor%20Object%20Reference) (OtherComp :type Primitive%20Component%20Object%20Reference) (OtherBodyIndex :type Integer) (bFromSweep :type Boolean) (SweepResult :type Hit%20Result%20Structure%20%28by%20ref%29))
  (Utilities|Casting|CastToBP_DungeonRunner OtherActor)
  (if (not (Variables|Default|GetIsDeactivated))
    (bind _spikemove (Timeline|Timeline PlayFromStart)
      (:Update
        (Transformation|SetRelativeLocation (Variables|Default|GetDamageZone) (Math|Vector|Lerp(Vector) "0.000000,0.000000,-40.000000" "0.000000,0.000000,40.000000" _spikemove) false false)))))

(event OnComponentBeginOverlap(DamageZone)
  (params (OverlappedComponent :type Primitive%20Component%20Object%20Reference) (OtherActor :type Actor%20Object%20Reference) (OtherComp :type Primitive%20Component%20Object%20Reference) (OtherBodyIndex :type Integer) (bFromSweep :type Boolean) (SweepResult :type Hit%20Result%20Structure%20%28by%20ref%29))
  (bind _asbp_dungeon_runner (Utilities|Casting|CastToBP_DungeonRunner OtherActor))
  (Utilities|FlowControl|DoOnce false :!label _label
    (:Completed
      (Default|TakeDamage _asbp_dungeon_runner (Variables|Default|GetTrapDamage))
      (Utilities|FlowControl|Delay 1.0)
      (goto _label Reset))))

(fn ConstructionScript
  (|CallParentFunction))