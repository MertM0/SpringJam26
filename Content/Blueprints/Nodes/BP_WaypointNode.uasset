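; Waypoint node that links to other nodes to form a graph and picks a weighted random next node.
; Construction script and BeginPlay both draw long-lived red debug arrows to each valid connected node.
; GetRandomConnectedNode excludes a given node, then runs a roulette-wheel pick over the remaining neighbors' CurrentWeight.
; It falls back to the first candidate when no positive weight matches.
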(event EventBeginPlay
  (for _array_element (Variables|Default|GetConnectedNodes)
    (Utilities|IsValid _array_element
      (:Is%20Valid
        (Rendering|Debug|DrawDebugArrow (Transformation|GetActorLocation) (Transformation|GetActorLocation _array_element) 99.0 "(R=1.000000,G=0.000000,B=0.000000,A=1.000000)" 9999999.0 3.0)))))

(fn ConstructionScript
  (for _array_element (Variables|Default|GetConnectedNodes)
    (Utilities|IsValid _array_element
      (:Is%20Valid
        (Rendering|Debug|DrawDebugArrow (Transformation|GetActorLocation) (Transformation|GetActorLocation _array_element) 99.0 "(R=1.000000,G=0.000000,B=0.000000,A=1.000000)" 9999999.0 3.0)))))

(fn GetRandomConnectedNode
  (params (NodeToIgnore :type BP%20Waypoint%20Node%20Object%20Reference))
  (bind _output_get (LocalVariables|SetValidNodes (Variables|Default|GetConnectedNodes)))
  (Utilities|Array|RemoveItem _output_get NodeToIgnore)
  (if (> (Utilities|Array|Length (LocalVariables|GetValidNodes)) 0)
    (LocalVariables|SetTotalWeight 0.0)
    (for _array_element (LocalVariables|GetValidNodes)
      (LocalVariables|SetTotalWeight (+ (LocalVariables|GetTotalWeight) (Variables|BP_WaypointNode_C|GetCurrentWeight _array_element))))
    (LocalVariables|SetRandomSpin (Math|Random|RandomFloatinRange 0.001 (LocalVariables|GetTotalWeight)))
    (LocalVariables|SetRunningSum 0.0)
    (for _array_element_2 (LocalVariables|GetValidNodes)
      (bind _output_get_2 (LocalVariables|SetRunningSum (+ (LocalVariables|GetRunningSum) (Variables|BP_WaypointNode_C|GetCurrentWeight _array_element_2))))
      (if (and (>= _output_get_2 (LocalVariables|GetRandomSpin)) (> (Variables|BP_WaypointNode_C|GetCurrentWeight _array_element_2) 0.0))
        (return _array_element_2)))
    (return (Utilities|Array|Get(acopy) (LocalVariables|GetValidNodes)))))