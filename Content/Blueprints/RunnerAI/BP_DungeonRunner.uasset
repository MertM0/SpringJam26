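; AI-controlled dungeon runner character that takes damage, falls into pits and respawns at the start node.
; A temporary shield absorbs one hit or fall; lethal damage ragdolls it, while pit falls play a shrinking timeline.
; Both deaths trigger a slow-motion kill cam, angled by line traces or fixed for pits, then clear the board and reset the AI.
; Tick feeds its location to a material parameter collection.
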(event Custom|PitFall
  (bind _returnvalue (Transformation|GetActorTransform))
  (bind _charactermovement (Variables|Character|GetCharacterMovement))
  (bind _mesh (Variables|Character|GetMesh))
  (if (Variables|Default|GetHasShield)
    (Variables|Default|SetHasShield false)
    (Rendering|SetVisibility (Variables|Default|GetDivineShield) false false)
    (Niagara|SpawnSystematLocation "/Game/Particles/P_Shield.P_Shield" (.location _returnvalue) (.rotation _returnvalue))
    (else
      (Components|Movement|StopMovementImmediately _charactermovement)
      (Pawn|Components|CharacterMovement|DisableMovement _charactermovement)
      (Physics|SetSimulatePhysics (Variables|Character|GetMesh) false)
      (Audio|PlaySoundatLocation "/Engine/EditorSounds/GamePreview/EndPlayInEditor.EndPlayInEditor" "0, 0, 0" "0, 0, 0" 1.0 1.0 0.0 0 0 0 0)
      (CallFunction|TriggerPitFallKillCam)
      (bind (_direction _z_offset _scale) (Timeline|T_PitFallAnimation PlayFromStart)
        (:Update
          (Transformation|SetRelativeLocation _mesh (Math|Vector|MakeVector 0.0 0.0 _z_offset) false false)
          (Transformation|SetRelativeScale3D _mesh (Math|Vector|MakeVector _scale _scale _scale)))))))

(event Custom|ApplyShieldBuff
  (Variables|Default|SetHasShield true)
  (Rendering|SetVisibility (Variables|Default|GetDivineShield) true false)
  (Utilities|FlowControl|RetriggerableDelay 3.0)
  (Variables|Default|SetHasShield false)
  (Rendering|SetVisibility (Variables|Default|GetDivineShield) false false))

(event Custom|CustomEvent
  ;[0.15 0.15 0.15 0.5] WIP
  (if (Utilities|Enum|Equal(Enum) (Variables|/Script/Engine.CharacterMovementComponent|GetMovementMode (Variables|Character|GetCharacterMovement)) "MOVE_Walking")
    (bind _returnvalue (Audio|SpawnSoundatLocation "/Game/Sounds/Running.Running" (Transformation|GetActorLocation) "0, 0, 0" 1.0 1.0 0.0 0 0))
    (Variables|Default|SetWalkSound _returnvalue)))

(event Custom|TriggerKillCam
  (Variables|Default|SetIsKillCamActive true)
  (Utilities|Time|SetGlobalTimeDilation 0.2)
  (bind _bestangle (CallFunction|GetSafestCameraAngle))
  (Transformation|SetRelativeRotation (Variables|Default|GetSpringArm) _bestangle false false)
  (Game|Player|SetViewTargetwithBlend (Game|GetPlayerController 0) self 0.15 "VTBlend_Linear" 0.0 false)
  (Utilities|FlowControl|Delay (* (Variables|Default|GetKillCamDuration) 0.2))
  (if (Variables|Default|GetIsKillCamActive)
    (CallFunction|EndKillCam)))

(event Custom|EndKillCam
  (Variables|Default|SetIsKillCamActive false)
  (Utilities|Time|SetGlobalTimeDilation 1.0)
  (bind _returnvalue (Actor|GetActorOfClass "/Game/Blueprints/BP_PlayerCamera.BP_PlayerCamera_C"))
  (Game|Player|SetViewTargetwithBlend (Game|GetPlayerController 0) _returnvalue 0.5 "VTBlend_Linear" 0.0 false)
  (Utilities|FlowControl|Delay 0.5)
  (CallFunction|Respawn))

(event Custom|TriggerPitFallKillCam
  (Variables|Default|SetIsKillCamActive true)
  (Utilities|Time|SetGlobalTimeDilation 0.2)
  (Transformation|SetRelativeRotation (Variables|Default|GetSpringArm) "-40.000000,90.000000,-90.000000" false false)
  (Game|Player|SetViewTargetwithBlend (Game|GetPlayerController 0) self 0.1 "VTBlend_Linear" 0.0 false)
  (Utilities|FlowControl|Delay (* (Variables|Default|GetKillCamDuration) 0.075))
  (if (Variables|Default|GetIsKillCamActive)
    (CallFunction|EndKillCam)))

(event EventBeginPlay
  ;[0.15 0.15 0.15 0.5] WIP
  (CallFunction|CustomEvent)
  (Utilities|Time|SetTimerbyEvent (delegate Custom|CustomEvent) 1.0 true))

(event EventTick
  (params (DeltaSeconds :type Float%20%28single-precision%29))
  (Rendering|Material|SetVectorParameterValue "/Game/Materials/Hole/Character_ParameterCollection.Character_ParameterCollection" "PlayerLocation" (Math|Conversions|ToLinearColor(Vector) (Transformation|GetActorLocation)) :!class /Script/Engine.KismetMaterialLibrary))

(fn ConstructionScript)

(fn TakeDamage
  (params (DamageAmount :type Integer))
  (bind _returnvalue (Transformation|GetActorTransform))
  (bind _returnvalue_2 (Transformation|GetActorTransform))
  (bind _charactermovement (Variables|Character|GetCharacterMovement))
  (bind _mesh (Variables|Character|GetMesh))
  (bind _walksound (Variables|Default|GetWalkSound))
  (if (Variables|Default|GetHasShield)
    (Variables|Default|SetHasShield false)
    (Rendering|SetVisibility (Variables|Default|GetDivineShield) false false)
    (Niagara|SpawnSystematLocation "/Game/Particles/P_Shield.P_Shield" (.location _returnvalue) (.rotation _returnvalue))
    (else
      (bind _output_get (Variables|Default|SetCurrentHealth (- (Variables|Default|GetCurrentHealth) DamageAmount)))
      (Audio|PlaySoundatLocation "/Game/Sounds/Death.Death" (Transformation|GetActorLocation) "0, 0, 0" 1.0 1.0 0.0 0 0 0 0)
      (Niagara|SpawnSystematLocation "/Game/Particles/P_Blood.P_Blood" (.location _returnvalue_2) (.rotation _returnvalue_2))
      (if (<= _output_get 0)
        (CallFunction|TriggerKillCam)
        ;[0.15 0.15 0.15 0.5] WIP
        (Audio|Components|Audio|Stop _walksound)
        (Components|DestroyComponent _walksound)
        (Pawn|Components|CharacterMovement|SetMovementMode (Variables|Character|GetCharacterMovement) "MOVE_None" 0)
        (Collision|SetCollisionEnabled (Variables|Collision|GetCapsuleComponent) "NoCollision")
        (Pawn|Components|CharacterMovement|DisableMovement _charactermovement)
        (Components|Movement|StopMovementImmediately _charactermovement)
        (bind _asbp_runner_aicontroller (Utilities|Casting|CastToBP_RunnerAIController (Pawn|GetController)))
        (AI|Logic|StopLogic (Variables|/Script/AIModule.AIController|GetBrainComponent _asbp_runner_aicontroller) "")
        (Physics|SetSimulatePhysics _mesh true)
        (Collision|SetCollisionProfileName _mesh "Ragdoll" true :!class /Script/Engine.PrimitiveComponent)))))

(fn Respawn
  (bind _mesh (Variables|Character|GetMesh))
  (Variables|/Script/Engine.SpringArmComponent|SetbDoCollisionTest (Variables|Default|GetSpringArm) true)
  (bind _asbp_player_camera (Utilities|Casting|CastToBP_PlayerCamera (Game|Player|GetPlayerPawn 0)))
  (Default|ClearBoard _asbp_player_camera)
  (bind _returnvalue (Actor|GetActorOfClass "/Game/Blueprints/Nodes/BP_StartNode.BP_StartNode_C"))
  (Transformation|SetActorLocation (Transformation|GetActorLocation _returnvalue) false true)
  (Collision|SetCollisionEnabled (Variables|Collision|GetCapsuleComponent) "QueryAndPhysics")
  (Physics|SetSimulatePhysics _mesh false)
  (Collision|SetCollisionProfileName _mesh "CharacterMesh" true :!class /Script/Engine.PrimitiveComponent)
  (Transformation|AttachComponentToComponent (Variables|Character|GetMesh) (Variables|Collision|GetCapsuleComponent) "None" "SnapToTarget" "SnapToTarget" "SnapToTarget" true)
  (Transformation|SetRelativeTransform (Variables|Character|GetMesh) (Math|Transform|MakeTransform "0.000000,0.000000,-90.000000" "0.000000,-90.000000,0.000000" "1.000000,1.000000,1.000000") false true)
  (Pawn|Components|CharacterMovement|SetMovementMode (Variables|Character|GetCharacterMovement) "MOVE_Walking" 0)
  (Variables|Default|SetCurrentHealth (Variables|Default|GetMaxHealth))
  (bind _asbp_runner_aicontroller (Utilities|Casting|CastToBP_RunnerAIController (Pawn|GetController)))
  (Default|ResetBrain _asbp_runner_aicontroller _returnvalue))

(fn GetSafestCameraAngle
  (bind _returnvalue (Transformation|GetActorLocation))
  (for _array_element (Utilities|Array|MakeArray "0, 0, 0" "0.000000,90.000000,0.000000" "0.000000,180.000000,0.000000" "0.000000,-90.000000,0.000000")
    (bind (_outhit _returnvalue_2) (Collision|LineTraceByChannel _returnvalue (+ _returnvalue (* (Math|Vector|GetForwardVector _array_element) 5e+02)) "TraceTypeQuery1" false 0 "None"))
    (if _returnvalue_2
      (if (> (.Distance (Collision|BreakHitResult _outhit)) (LocalVariables|GetMaxDistance))
        (LocalVariables|SetMaxDistance (.Distance (Collision|BreakHitResult _outhit)))
        (bind _output_get (LocalVariables|SetBestRot (Math|Rotator|MakeRotator (.Roll (Math|Rotator|BreakRotator _array_element)) (.Pitch (Math|Rotator|BreakRotator _array_element)) (+ (.Yaw (Math|Rotator|BreakRotator _array_element)) 1.8e+02))))
        (return _output_get)))))