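; Base actor for a clickable 3D main menu button, with a mesh and a WBP_MenuText widget whose text is set at construction and BeginPlay.
; Cursor hover sets mesh overlay and widget materials, and a timeline scales the widget up, reversing on exit.
; A click blocks interaction through BP_MainMenuController, blends the camera view to the button, then calls ButtonAction, an empty hook.
; Hover and click responses are ignored while interaction is blocked.
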(event OnEndCursorOver(StaticMesh)
  (params (TouchedComponent :type Primitive%20Component%20Object%20Reference))
  (if (not (Variables|/Game/MainMenu_Widget/BP_MainMenuController.BP_MainMenuController_C|GetbIsInteractionBlocked (Variables|Default|GetAs%20BP%20Main%20Menu%20Controller)))
    (Rendering|Material|SetOverlayMaterial (Variables|Default|GetStaticMesh) 0 :!class /Script/Engine.MeshComponent)
    (Rendering|Material|SetMaterial (Variables|Default|GetWidget) 0 0)
    (bind _alpha (Timeline|TM_HoverAnimation Reverse)
      (:Update
        (Transformation|SetRelativeScale3D (Variables|Default|GetWidget) (Math|Vector|Lerp(Vector) (Variables|Default|GetWidgetScale) (* (Variables|Default|GetWidgetScale) 1.5) _alpha))))))

(event OnClicked(StaticMesh)
  (params (TouchedComponent :type Primitive%20Component%20Object%20Reference) (ButtonPressed :type Key%20Structure))
  (bind _as_bp_main_menu_controller (Variables|Default|GetAs%20BP%20Main%20Menu%20Controller))
  (if (not (Variables|/Game/MainMenu_Widget/BP_MainMenuController.BP_MainMenuController_C|GetbIsInteractionBlocked _as_bp_main_menu_controller))
    (Variables|/Game/MainMenu_Widget/BP_MainMenuController.BP_MainMenuController_C|SetbIsInteractionBlocked _as_bp_main_menu_controller true)
    (Game|Player|SetViewTargetwithBlend (Game|GetPlayerController 0) self 1.0 "VTBlend_EaseInOut" 2.0 false)
    (Utilities|FlowControl|Delay 1.0)
    (CallFunction|ButtonAction)))

(event OnBeginCursorOver(StaticMesh)
  (params (TouchedComponent :type Primitive%20Component%20Object%20Reference))
  (if (not (Variables|/Game/MainMenu_Widget/BP_MainMenuController.BP_MainMenuController_C|GetbIsInteractionBlocked (Variables|Default|GetAs%20BP%20Main%20Menu%20Controller)))
    (Rendering|Material|SetOverlayMaterial (Variables|Default|GetStaticMesh) 0 :!class /Script/Engine.MeshComponent)
    (Rendering|Material|SetMaterial (Variables|Default|GetWidget) 0 0)
    (bind _alpha (Timeline|TM_HoverAnimation PlayFromStart)
      (:Update
        (Transformation|SetRelativeScale3D (Variables|Default|GetWidget) (Math|Vector|Lerp(Vector) (Variables|Default|GetWidgetScale) (* (Variables|Default|GetWidgetScale) 1.5) _alpha))))))

(event Custom|ButtonAction)

(event EventBeginPlay
  (bind _aswbp_menu_text (Utilities|Casting|CastToWBP_MenuText (UserInterface|GetWidget (Variables|Default|GetWidget))))
  (Default|SetDynamicText _aswbp_menu_text (Variables|Default|GetText))
  (Variables|Default|SetMenuText (Variables|/Game/MainMenu_Widget/WBP_MenuText.WBP_MenuText_C|GetMenuText _aswbp_menu_text))
  (Variables|Default|SetWidgetScale (Variables|/Script/Engine.SceneComponent|GetRelativeScale3D (Variables|Default|GetWidget)))
  (bind _asbp_main_menu_controller (Utilities|Casting|CastToBP_MainMenuController (Game|GetPlayerController 0)))
  (Variables|Default|SetAs%20BP%20Main%20Menu%20Controller _asbp_main_menu_controller))

(fn ConstructionScript
  (bind _aswbp_menu_text (Utilities|Casting|CastToWBP_MenuText (UserInterface|GetWidget (Variables|Default|GetWidget))))
  (Default|SetDynamicText _aswbp_menu_text (Variables|Default|GetText)))