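; BP_MainMenuCredits is a main menu button, named for credits, with a static mesh and a 3D widget component.
; ButtonAction creates the WidgetToOpen class for the first player controller and adds it to the viewport.
; ResetButton clears the mesh overlay, sets the widget material and plays a timeline in reverse from the end, lerping widget scale from enlarged back toward its base size.
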(event Custom|Reset%20Button
  (bind _widgetscale (Variables|Default|GetWidgetScale))
  (Rendering|Material|SetOverlayMaterial (Variables|Default|GetStaticMesh) 0 :!class /Script/Engine.MeshComponent)
  (Rendering|Material|SetMaterial (Variables|Default|GetWidget) 0 "/Game/MainMenu_Widget/M_WidgetMaterial.M_WidgetMaterial")
  (bind _newtrack_0 (Timeline|Timeline ReverseFromEnd)
    (:Update
      (Transformation|SetRelativeScale3D (Variables|Default|GetWidget) (Math|Vector|Lerp(Vector) _widgetscale (* _widgetscale 1.5) _newtrack_0)))))

(event EventBeginPlay
  (|CallParentFunction) ; This node is disabled and will not be called.\nDrag off pins to build functionality.
)

(event EventButtonAction
  (bind _returnvalue (UserInterface|CreateWidget (Variables|Default|GetWidgetToOpen) (Game|GetPlayerController 0)))
  (UserInterface|Viewport|AddtoViewport _returnvalue 0))

(fn ConstructionScript
  (|CallParentFunction))